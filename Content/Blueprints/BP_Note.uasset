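; BP_Note is a note actor that travels along one of four spline lanes, likely for a rhythm game.
; On BeginPlay, the MoveNote timeline starts and drives the note's progress along the Left, Bottom, Top or Right spline of SplineRef, selected by NoteType.
; Each update maps the timeline alpha to spline distance and applies world location and rotation at unit scale, without sweeping.
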(event EventBeginPlay
  (bind _splineref (Variables|Default|GetSplineRef))
  (bind _notetype (Variables|Default|GetNoteType))
  (bind _spline_bottom (Variables|/Game/Blueprints/BP_RythmeSpline.BP_RythmeSpline_C|GetSpline_Bottom _splineref))
  (bind _spline_left (Variables|/Game/Blueprints/BP_RythmeSpline.BP_RythmeSpline_C|GetSpline_Left _splineref))
  (bind _spline_right (Variables|/Game/Blueprints/BP_RythmeSpline.BP_RythmeSpline_C|GetSpline_Right _splineref))
  (bind _spline_top (Variables|/Game/Blueprints/BP_RythmeSpline.BP_RythmeSpline_C|GetSpline_Top _splineref))
  (bind _returnvalue (Utilities|Select :Index _notetype :NewEnumerator0 _spline_left :NewEnumerator1 _spline_bottom :NewEnumerator2 _spline_top :NewEnumerator3 _spline_right))
  (bind _newtrack_0 (Timeline|MoveNote Play)
    (:Update
      (Transformation|SetActorTransform (Math|Transform|MakeTransform (Spline|GetLocationatDistanceAlongSpline _returnvalue (Math|Float|Lerp 0.0 (Spline|GetSplineLength _returnvalue) _newtrack_0) "World") (Spline|GetRotationatDistanceAlongSpline _returnvalue (Math|Float|Lerp 0.0 (Spline|GetSplineLength _returnvalue) _newtrack_0) "World"))))))

(fn ConstructionScript)