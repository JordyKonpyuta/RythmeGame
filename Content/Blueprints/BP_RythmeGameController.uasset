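; BP_RythmeGameController handles input for a rhythm game, covering only the right-hand lane via the Right and D keys.
; On press, it takes the first BP_Note overlapping the spline actor's SphereRight and measures its signed world X offset from ArrowSphereRight.
; It passes that offset and note to RythmeSplineRef's VerifyInput, checking that the spline reference is valid but not that any note overlaps.
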(event Input|KeyboardEvents|Z
  (params (Key :type Key%20Structure :default "None")))

(event Input|KeyboardEvents|Down
  (params (Key :type Key%20Structure :default "None")))

(event Input|KeyboardEvents|S
  (params (Key :type Key%20Structure :default "None")))

(event Input|KeyboardEvents|Left
  (params (Key :type Key%20Structure :default "None")))

(event Input|KeyboardEvents|Q
  (params (Key :type Key%20Structure :default "None")))

(event Input|KeyboardEvents|Right
  (params (Key :type Key%20Structure :default "None"))
  (bind _rythmesplineref (Variables|Default|GetRythmeSplineRef))
  (bind _sphere_right (Variables|/Game/Blueprints/BP_RythmeSpline.BP_RythmeSpline_C|GetSphere_Right _rythmesplineref))
  (bind _overlappingactors (Collision|GetOverlappingActors _sphere_right "/Game/Blueprints/BP_Note.BP_Note_C" :!class /Script/Engine.PrimitiveComponent))
  (bind _output (Utilities|Array|Get(acopy) _overlappingactors))
  (:Pressed
    (Utilities|IsValid _rythmesplineref
      (:Is%20Valid
        (Default|VerifyInput (Variables|Default|GetRythmeSplineRef) (.x (- (Transformation|GetActorLocation _output) (Transformation|GetWorldLocation (Variables|/Game/Blueprints/BP_RythmeSpline.BP_RythmeSpline_C|GetArrow_Sphere_Right _rythmesplineref)))) (.AsBP%20Note (Utilities|Casting|CastToBP_Note _output)))))))

(event Input|KeyboardEvents|D
  (params (Key :type Key%20Structure :default "None"))
  (bind _rythmesplineref (Variables|Default|GetRythmeSplineRef))
  (bind _sphere_right (Variables|/Game/Blueprints/BP_RythmeSpline.BP_RythmeSpline_C|GetSphere_Right _rythmesplineref))
  (bind _overlappingactors (Collision|GetOverlappingActors _sphere_right "/Game/Blueprints/BP_Note.BP_Note_C" :!class /Script/Engine.PrimitiveComponent))
  (bind _output (Utilities|Array|Get(acopy) _overlappingactors))
  (:Pressed
    (Utilities|IsValid _rythmesplineref
      (:Is%20Valid
        (Default|VerifyInput (Variables|Default|GetRythmeSplineRef) (.x (- (Transformation|GetActorLocation _output) (Transformation|GetWorldLocation (Variables|/Game/Blueprints/BP_RythmeSpline.BP_RythmeSpline_C|GetArrow_Sphere_Right _rythmesplineref)))) (.AsBP%20Note (Utilities|Casting|CastToBP_Note _output)))))))

(event Input|KeyboardEvents|Up
  (params (Key :type Key%20Structure :default "None")))

(fn ConstructionScript)