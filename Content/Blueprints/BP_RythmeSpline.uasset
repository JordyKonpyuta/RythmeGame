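; Rhythm game lane actor that spawns directional notes in time with music and grades hits.
; StartSequence registers it with BP_RythmeGameController, plays a MetaSound and watches its CuePoint_Direction output.
; Each cue's suffix (Top, Bottom, Right, Left) spawns a typed BP_Note at the matching arrow.
; VerifyInput grades the negated distance as Perfect, Great, Good or Miss, prints the result and destroys the note.
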(event Custom|StartSequence
  (Utilities|FlowControl|Sequence
    (:then_0
      (bind _asbp_rythme_game_controller (Utilities|Casting|CastToBP_RythmeGameController (Game|GetPlayerController 0)))
      (Variables|/Game/Blueprints/BP_RythmeGameController.BP_RythmeGameController_C|SetRythmeSplineRef _asbp_rythme_game_controller self))
    (:then_1
      (bind _returnvalue (Audio|SpawnSound2D (Variables|Default|GetSoundToPlay) 1.0 1.0 0.0 0))
      (bind _output_get (Variables|Default|SetAudio _returnvalue))
      (Class|AudioParameterControllerInterface|SetTriggerParameter _output_get "On Play")
      (MetaSoundOutput|WatchOutput (WorldSubsystems|GetMetaSoundOutputSubsystem) (Variables|Default|GetAudio) "CuePoint_Direction" (delegate Custom|SpawnNoteOnGoodLine) "None" "None" :!class /Script/MetasoundEngine.MetaSoundOutputSubsystem))))

(event Custom|SpawnNoteOnGoodLine
  (params (OutputName :type Name) (Output :type Meta%20Sound%20Output%20Structure%20%28by%20ref%29))
  (bind _returnvalue (Class|MetasoundOutputBlueprintAccess|GetString Output))
  (for (_array_element _array_index) (Utilities|Array|MakeArray (Utilities|Enum|Equal(Enum) (.RightS (Utilities|String|Split _returnvalue "_")) "Top") (Utilities|Enum|Equal(Enum) (.RightS (Utilities|String|Split _returnvalue "_")) "Bottom") (Utilities|Enum|Equal(Enum) (.RightS (Utilities|String|Split _returnvalue "_")) "Right") (Utilities|Enum|Equal(Enum) (.RightS (Utilities|String|Split _returnvalue "_")) "Left"))
    (if _array_element
      (Game|SpawnActorfromClass "/Game/Blueprints/BP_Note.BP_Note_C" (Transformation|GetWorldTransform (Utilities|Array|Get(acopy) (Utilities|Array|MakeArray (Variables|Default|GetArrow_Top) (Variables|Default|GetArrow_Bottom) (Variables|Default|GetArrow_Right) (Variables|Default|GetArrow_Left)) _array_index)) "Undefined" "MultiplyWithRoot" 0 (Utilities|Select :Index _array_index :Option%200 "NewEnumerator2" :Option%201 "NewEnumerator1" :Option%202 "NewEnumerator3" :Option%203 "NewEnumerator0") self 0))))

(event Custom|VerifyInput
  (params (Distance :type Float%20%28double-precision%29) (NoteToVerify :type BP%20Note%20Object%20Reference))
  (bind _returnvalue (* Distance -1.0))
  (if (<= _returnvalue 35.0)
    (Development|PrintString "Perfect !")
    (Actor|DestroyActor NoteToVerify)
    (elif (and (> _returnvalue 35.0) (<= _returnvalue 65.0))
      (Development|PrintString "Great !")
      (Actor|DestroyActor NoteToVerify)
      (elif (and (> _returnvalue 65.0) (<= _returnvalue 1.6e+02))
        (Development|PrintString "Good !")
        (Actor|DestroyActor NoteToVerify)
        (else
          (Development|PrintString "Miss !")
          (Actor|DestroyActor NoteToVerify))))))

(fn ConstructionScript)