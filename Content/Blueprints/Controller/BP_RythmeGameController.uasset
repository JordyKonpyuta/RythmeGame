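; Player controller for a four-direction rhythm game that creates the main menu, handles input and keeps score.
; Direction inputs pulse RythmeSplineRef and pass it the first overlapping note's X offset from that lane's arrow for verification.
; AddScore tracks combo, with a ratio rising every ten hits, and rank compares score to a simulated maximum for the selected track.
; Reset and quit inputs stop notes and audio, then fade to restart or track selection.
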(event Custom|AddScore
  (params (ScoreToAdd :type Integer))
  (bind _rythmesplineref (Variables|Default|GetRythmeSplineRef))
  (bind _ui_ref (Variables|/Game/Blueprints/RythmePart/BP_RythmeSpline.BP_RythmeSpline_C|GetUI_Ref _rythmesplineref))
  ;[0.15 0.15 0.15 0.5] Scoring System
  (Variables|Default|SetScore (+ (Variables|Default|GetScore) (select (> (Variables|Default|GetCombo) 0) (Math|Float|Truncate (* (Variables|Default|GetCombo) (Variables|Default|GetComboRatio))) ScoreToAdd)))
  (Default|SetScoreTexts (Variables|/Game/Blueprints/RythmePart/BP_RythmeSpline.BP_RythmeSpline_C|GetUI_Ref (Variables|Default|GetRythmeSplineRef)) (select (> (Variables|Default|GetCombo) 0) (Math|Float|Truncate (* (Variables|Default|GetCombo) (Variables|Default|GetComboRatio))) ScoreToAdd))
  (bind _result (Math|Integer|IncrementInt (Variables|Default|GetCombo))
    (:%20%20
      (Default|SetComboRangeCharacter _ui_ref)
      (Default|DisplayDancers _ui_ref)
      (Default|FeedbackGameplay (Variables|Default|GetMainMenuRef))
      (Utilities|FlowControl|Sequence
        (:then_0
          (if (== (Math|Integer|%(Integer) _result 10) 0)
            (Variables|Default|SetComboRatio (+ (Variables|Default|GetComboRatio) 0.5))))
        (:then_1
          (if (> (Variables|Default|GetCombo) (Variables|Default|GetMaxCombo))
            (Variables|Default|SetMaxCombo (Variables|Default|GetCombo))))))))

(event Custom|SetAllVariablesToZero
  (bind _amountofeachnotesuccess (Variables|Default|GetAmountOfEachNoteSuccess))
  (bind _rythmesplineref (Variables|Default|GetRythmeSplineRef))
  (bind _ui_ref (Variables|/Game/Blueprints/RythmePart/BP_RythmeSpline.BP_RythmeSpline_C|GetUI_Ref _rythmesplineref))
  ;[0.15 0.15 0.15 0.5] Set all variables to zero
  (Variables|Default|SetScore 0)
  (Variables|Default|SetCombo 0)
  (Variables|Default|SetComboRatio 1.5)
  (Variables|Default|SetNotesHitted 0)
  (Variables|Default|SetMaxCombo 0)
  (for (_ _array_index) _amountofeachnotesuccess
    (Utilities|Array|SetArrayElem _amountofeachnotesuccess _array_index 0 true)
    (Default|SetScoreTexts _ui_ref)
    (Rendering|Components|TextRender|SetText (Variables|/Game/Blueprints/RythmePart/WBP_Gameplay.WBP_Gameplay_C|GetText_TrackProgress _ui_ref) "0 %")))

(event Input|EnhancedActionEvents|EnhancedInputActionIA_Left
  (params (ActionValue :type Boolean) (ElapsedSeconds :type Float%20%28double-precision%29) (TriggeredSeconds :type Float%20%28double-precision%29) (InputAction :type Input%20Action%20Object%20Reference :default "/Game/Blueprints/Controller/Inputs/IA_Left.IA_Left"))
  (bind _rythmesplineref (Variables|Default|GetRythmeSplineRef))
  (bind _sphere_left (Variables|/Game/Blueprints/RythmePart/BP_RythmeSpline.BP_RythmeSpline_C|GetSphere_Left _rythmesplineref))
  (bind _overlappingactors (Collision|GetOverlappingActors _sphere_left "/Game/Blueprints/RythmePart/BP_Note.BP_Note_C" :!class /Script/Engine.PrimitiveComponent))
  (bind _output (Utilities|Array|Get(acopy) _overlappingactors))
  (bind _asbp_note (Utilities|Casting|CastToBP_Note _output))
  ;[0.15 0.15 0.15 0.5] Inputs Directions
  (Utilities|IsValid _rythmesplineref
    (:Is%20Valid
      (Default|PulsingEnteredInput _rythmesplineref "NewEnumerator0")
      (Utilities|IsValid _asbp_note
        (:Is%20Valid
          (Default|VerifyInput (Variables|Default|GetRythmeSplineRef) (.x (- (Transformation|GetActorLocation _output) (Transformation|GetWorldLocation (Variables|/Game/Blueprints/RythmePart/BP_RythmeSpline.BP_RythmeSpline_C|GetArrow_Sphere_Left _rythmesplineref)))) _asbp_note))))))

(event Input|EnhancedActionEvents|EnhancedInputActionIA_Reset
  (params (ActionValue :type Boolean) (ElapsedSeconds :type Float%20%28double-precision%29) (TriggeredSeconds :type Float%20%28double-precision%29) (InputAction :type Input%20Action%20Object%20Reference :default "/Game/Blueprints/Controller/Inputs/IA_Reset.IA_Reset"))
  (bind _mainmenuref (Variables|Default|GetMainMenuRef))
  (bind _rythmesplineref (Variables|Default|GetRythmeSplineRef))
  (bind _mainmenuref_2 (Variables|Default|GetMainMenuRef))
  ;[0.15 0.15 0.15 0.5] Input Reset Track
  (Variables|Default|SetIsResetting true)
  (Default|CallDestroyAllNotes)
  (Audio|Components|Audio|Stop (Variables|/Game/Blueprints/RythmePart/BP_RythmeSpline.BP_RythmeSpline_C|GetAudio _rythmesplineref))
  (Audio|Components|Audio|Stop (Variables|/Game/Blueprints/RythmePart/BP_RythmeSpline.BP_RythmeSpline_C|GetAudioPreview _rythmesplineref))
  (Components|Animation|PlayAnimation _mainmenuref_2 (Variables|/Game/Blueprints/RythmePart/WBP_MainMenu.WBP_MainMenu_C|GetFadeToBlack _mainmenuref_2) 0.0
    (:Finished
      (CallFunction|SetAllVariablestoZero)
      (Components|Animation|PlayAnimation _mainmenuref (Variables|/Game/Blueprints/RythmePart/WBP_MainMenu.WBP_MainMenu_C|GetFadeToBlack _mainmenuref) 0.0 1 "Reverse"
        (:Finished
          (Widget|SetVisibility (Variables|/Game/Blueprints/RythmePart/WBP_MainMenu.WBP_MainMenu_C|GetImage_FadeToBlack (Variables|Default|GetMainMenuRef)) "Collapsed")
          (Utilities|FlowControl|Delay 1.0)
          (Default|StartSequence (Variables|Default|GetRythmeSplineRef)))))))

(event Input|EnhancedActionEvents|EnhancedInputActionIA_Right
  (params (ActionValue :type Boolean) (ElapsedSeconds :type Float%20%28double-precision%29) (TriggeredSeconds :type Float%20%28double-precision%29) (InputAction :type Input%20Action%20Object%20Reference :default "/Game/Blueprints/Controller/Inputs/IA_Right.IA_Right"))
  (bind _rythmesplineref (Variables|Default|GetRythmeSplineRef))
  (bind _sphere_right (Variables|/Game/Blueprints/RythmePart/BP_RythmeSpline.BP_RythmeSpline_C|GetSphere_Right _rythmesplineref))
  (bind _overlappingactors (Collision|GetOverlappingActors _sphere_right "/Game/Blueprints/RythmePart/BP_Note.BP_Note_C" :!class /Script/Engine.PrimitiveComponent))
  (bind _output (Utilities|Array|Get(acopy) _overlappingactors))
  (bind _asbp_note (Utilities|Casting|CastToBP_Note _output))
  ;[0.15 0.15 0.15 0.5] Inputs Directions
  (Utilities|IsValid _rythmesplineref
    (:Is%20Valid
      (Default|PulsingEnteredInput _rythmesplineref "NewEnumerator3")
      (Utilities|IsValid _asbp_note
        (:Is%20Valid
          (Default|VerifyInput (Variables|Default|GetRythmeSplineRef) (.x (- (Transformation|GetActorLocation _output) (Transformation|GetWorldLocation (Variables|/Game/Blueprints/RythmePart/BP_RythmeSpline.BP_RythmeSpline_C|GetArrow_Sphere_Right _rythmesplineref)))) _asbp_note))))))

(event Input|EnhancedActionEvents|EnhancedInputActionIA_Up
  (params (ActionValue :type Boolean) (ElapsedSeconds :type Float%20%28double-precision%29) (TriggeredSeconds :type Float%20%28double-precision%29) (InputAction :type Input%20Action%20Object%20Reference :default "/Game/Blueprints/Controller/Inputs/IA_Up.IA_Up"))
  (bind _rythmesplineref (Variables|Default|GetRythmeSplineRef))
  (bind _sphere_top (Variables|/Game/Blueprints/RythmePart/BP_RythmeSpline.BP_RythmeSpline_C|GetSphere_Top _rythmesplineref))
  (bind _overlappingactors (Collision|GetOverlappingActors _sphere_top "/Game/Blueprints/RythmePart/BP_Note.BP_Note_C" :!class /Script/Engine.PrimitiveComponent))
  (bind _output (Utilities|Array|Get(acopy) _overlappingactors))
  (bind _asbp_note (Utilities|Casting|CastToBP_Note _output))
  ;[0.15 0.15 0.15 0.5] Inputs Directions
  (Utilities|IsValid _rythmesplineref
    (:Is%20Valid
      (Default|PulsingEnteredInput _rythmesplineref "NewEnumerator2")
      (Utilities|IsValid _asbp_note
        (:Is%20Valid
          (Default|VerifyInput (Variables|Default|GetRythmeSplineRef) (.x (- (Transformation|GetActorLocation _output) (Transformation|GetWorldLocation (Variables|/Game/Blueprints/RythmePart/BP_RythmeSpline.BP_RythmeSpline_C|GetArrow_Sphere_Top _rythmesplineref)))) _asbp_note))))))

(event Input|EnhancedActionEvents|EnhancedInputActionIA_Down
  (params (ActionValue :type Boolean) (ElapsedSeconds :type Float%20%28double-precision%29) (TriggeredSeconds :type Float%20%28double-precision%29) (InputAction :type Input%20Action%20Object%20Reference :default "/Game/Blueprints/Controller/Inputs/IA_Down.IA_Down"))
  (bind _rythmesplineref (Variables|Default|GetRythmeSplineRef))
  (bind _sphere_bottom (Variables|/Game/Blueprints/RythmePart/BP_RythmeSpline.BP_RythmeSpline_C|GetSphere_Bottom _rythmesplineref))
  (bind _overlappingactors (Collision|GetOverlappingActors _sphere_bottom "/Game/Blueprints/RythmePart/BP_Note.BP_Note_C" :!class /Script/Engine.PrimitiveComponent))
  (bind _output (Utilities|Array|Get(acopy) _overlappingactors))
  (bind _asbp_note (Utilities|Casting|CastToBP_Note _output))
  ;[0.15 0.15 0.15 0.5] Inputs Directions
  (Utilities|IsValid _rythmesplineref
    (:Is%20Valid
      (Default|PulsingEnteredInput _rythmesplineref "NewEnumerator1")
      (Utilities|IsValid _asbp_note
        (:Is%20Valid
          (Default|VerifyInput (Variables|Default|GetRythmeSplineRef) (.x (- (Transformation|GetActorLocation _output) (Transformation|GetWorldLocation (Variables|/Game/Blueprints/RythmePart/BP_RythmeSpline.BP_RythmeSpline_C|GetArrow_Sphere_Bottom _rythmesplineref)))) _asbp_note))))))

(event Input|EnhancedActionEvents|EnhancedInputActionIA_Quit
  (params (ActionValue :type Boolean) (ElapsedSeconds :type Float%20%28double-precision%29) (TriggeredSeconds :type Float%20%28double-precision%29) (InputAction :type Input%20Action%20Object%20Reference :default "/Game/Blueprints/Controller/Inputs/IA_Quit.IA_Quit"))
  (bind _mainmenuref (Variables|Default|GetMainMenuRef))
  (bind _mainmenuref_2 (Variables|Default|GetMainMenuRef))
  (bind _rythmesplineref (Variables|Default|GetRythmeSplineRef))
  (bind _mainmenuref_3 (Variables|Default|GetMainMenuRef))
  (bind _audio (Variables|/Game/Blueprints/RythmePart/BP_RythmeSpline.BP_RythmeSpline_C|GetAudio _rythmesplineref))
  (bind _audiopreview (Variables|/Game/Blueprints/RythmePart/BP_RythmeSpline.BP_RythmeSpline_C|GetAudioPreview _rythmesplineref))
  ;[0.15 0.15 0.15 0.5] Input Quit Track
  (Variables|Default|SetIsResetting true)
  (Default|CallDestroyAllNotes)
  (Utilities|IsValid _audio
    (:Is%20Valid
      (Audio|Components|Audio|Stop _audio))
    (:Is%20Not%20Valid
      _))
  (Utilities|IsValid _audiopreview
    (:Is%20Valid
      (Audio|Components|Audio|Stop _audiopreview))
    (:Is%20Not%20Valid
      _))
  (Components|Animation|PlayAnimation _mainmenuref (Variables|/Game/Blueprints/RythmePart/WBP_MainMenu.WBP_MainMenu_C|GetFadeToBlack _mainmenuref) 0.0
    (:Finished
      (Input|SetInputModeUIOnly self (Variables|Default|GetMainMenuRef) "DoNotLock" true)
      (Variables|Default|SetbShowMouseCursor true)
      (Default|CheckSelectedTrack _mainmenuref_2)
      (Default|SetPreviewSound _mainmenuref_2)
      (Class|WidgetSwitcher|SetActiveWidgetIndex (Variables|/Game/Blueprints/RythmePart/WBP_MainMenu.WBP_MainMenu_C|GetWS_MainMenu _mainmenuref_2) 1)
      (Components|Animation|PlayAnimation _mainmenuref_3 (Variables|/Game/Blueprints/RythmePart/WBP_MainMenu.WBP_MainMenu_C|GetPopUp_TrackSelection _mainmenuref_3) 0.0
        (:Finished
          (Default|DisplayCurrentTrack _mainmenuref_2))))))

(event EventBeginPlay
  (bind _self self)
  (bind _returnvalue (PlayerController|LocalPlayerSubsystems|GetEnhancedInputLocalPlayerSubsystem _self))
  (bind _returnvalue_2 (Class|EnhancedInputSubsystemInterface|GetUserSettings _returnvalue))
  ;[0.15 0.15 0.15 0.5] Begin Play
  (Utilities|FlowControl|Sequence
    (:then_0
      (Input|AddMappingContext _returnvalue "/Game/Blueprints/Controller/IMC_Base.IMC_Base" 0 "(bIgnoreAllPressedKeysUntilRelease=True,bForceImmediately=False,bNotifyUserSettings=False)")
      (if (not (Class|EnhancedInputUserSettings|IsMappingContextRegistered _returnvalue_2 "/Game/Blueprints/Controller/IMC_Base.IMC_Base"))
        (Class|EnhancedInputUserSettings|RegisterInputMappingContext _returnvalue_2 "/Game/Blueprints/Controller/IMC_Base.IMC_Base")))
    (:then_1
      (bind _returnvalue_3 (UserInterface|CreateWidget "/Game/Blueprints/RythmePart/WBP_MainMenu.WBP_MainMenu_C"))
      (bind _output_get (Variables|Default|SetMainMenuRef _returnvalue_3))
      (UserInterface|Viewport|AddtoViewport _output_get 0))))

(fn ConstructionScript)

(fn CalculateHigherScorePossible
  (bind _tempcombo (LocalVariables|GetTempCombo))
  (for _index (range 0 (Utilities|Struct|BreakS_Tracks (Variables|Default|GetSelectedTrack)))
    (Utilities|FlowControl|Sequence
      (:then_0
        (bind _result (Math|Integer|IncrementInt (LocalVariables|GetTempCombo))
          (:%20%20
            (if (== (Math|Integer|%(Integer) _result 10) 0)
              (LocalVariables|SetTempComboRatio (+ (LocalVariables|GetTempComboRatio) 0.5))))))
      (:then_1
        (LocalVariables|SetTempScore (* (+ (LocalVariables|GetTempScore) 500) (select (> _tempcombo 0) (Math|Float|Truncate (* _tempcombo (LocalVariables|GetTempComboRatio))) 1))))))
  (return (LocalVariables|GetTempScore)))

(fn VerifyRankObtained
  (bind _higherscorepossible (CallFunction|CalculateHigherScorePossible))
  (return (select (== (Variables|Default|GetScore) _higherscorepossible) 6 (select (>= (Variables|Default|GetScore) (Math|Float|Truncate (* _higherscorepossible 0.8))) 5 (select (>= (Variables|Default|GetScore) (Math|Float|Truncate (* _higherscorepossible 0.6))) 4 (select (>= (Variables|Default|GetScore) (Math|Float|Truncate (* _higherscorepossible 0.5))) 3 (select (>= (Variables|Default|GetScore) (Math|Float|Truncate (* _higherscorepossible 0.4))) 2 (select (>= (Variables|Default|GetScore) (Math|Float|Truncate (* _higherscorepossible 0.2))) 1 (select (< (Variables|Default|GetScore) (Math|Float|Truncate (* _higherscorepossible 0.2))) 0 0)))))))))