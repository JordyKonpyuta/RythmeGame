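; BP_RythmeGameInstance is the game instance for a rhythm game that loads or creates the persistent save data on startup.
; On Init it loads the BP_RythmeSaveGame from the "Global" slot and keeps it in SaveGame.
; If no save exists, it creates one, seeds parallel high score, name and best rank arrays with a default entry per DT_Tracks row, then writes it to the slot.
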(event EventInit
  (bind _returnvalue (SaveGame|DoesSaveGameExist "Global"))
  (if _returnvalue
    (bind _returnvalue_2 (SaveGame|LoadGamefromSlot "Global"))
    (bind _asbp_rythme_save_game (Utilities|Casting|CastToBP_RythmeSaveGame _returnvalue_2))
    (Variables|Default|SetSaveGame _asbp_rythme_save_game)
    (else
      (bind _returnvalue_3 (SaveGame|CreateSaveGameObject "/Game/Blueprints/Controller/BP_RythmeSaveGame.BP_RythmeSaveGame_C"))
      (bind _output_get (Variables|Default|SetSaveGame _returnvalue_3))
      (bind _outrownames (DataTable|GetDataTableRowNames "/Game/Blueprints/Datas/DT_Tracks.DT_Tracks"))
      (for _array_element _outrownames
        (Utilities|Array|Add (Variables|/Game/Blueprints/Controller/BP_RythmeSaveGame.BP_RythmeSaveGame_C|GetHigherScores (Variables|Default|GetSaveGame)) 0)
        (Utilities|Array|Add (Variables|/Game/Blueprints/Controller/BP_RythmeSaveGame.BP_RythmeSaveGame_C|GetNames (Variables|Default|GetSaveGame)) "")
        (Utilities|Array|Add (Variables|/Game/Blueprints/Controller/BP_RythmeSaveGame.BP_RythmeSaveGame_C|GetBestRanks (Variables|Default|GetSaveGame)) 0))
      (SaveGame|SaveGametoSlot _output_get "Global"))))