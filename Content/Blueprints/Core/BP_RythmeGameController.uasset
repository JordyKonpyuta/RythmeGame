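; Player controller for the rhythm game that handles input, scoring and ranking, and opens the intro widget.
; Debounced directional inputs pass the overlapping note and its X offset in that lane's sphere to the spline actor for verification.
; AddScore applies a combo multiplier and feeds UI feedback and Nozomi/Boken scores, while rank compares unmultiplied score to the track maximum.
; Reset and quit stop audio and clear notes behind a fade, then restart or return to track selection.
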(event Custom|AddScore
  (params (ScoreToAdd :type Integer) (NoteSuccess :type Integer))
  (bind _rythmesplineref (Variables|References|GetRythmeSplineRef))
  (bind _mainmenuref (Variables|References|GetMainMenuRef))
  (bind _ui_ref (Variables|/Game/Blueprints/RythmePart/BP_RythmeSpline.BP_RythmeSpline_C|GetUI_Ref _rythmesplineref))
  ;[0.15 0.15 0.15 0.5] Scoring System
  (Variables|Scoring|SetScore (+ (Variables|Scoring|GetScore) (select (> (Variables|Scoring|GetCombo) 0) (Math|Float|Truncate (* (Variables|Scoring|GetCombo) (Variables|Scoring|GetComboRatio) ScoreToAdd)) ScoreToAdd)))
  (Variables|Scoring|SetRankScore (+ (Variables|Scoring|GetRankScore) ScoreToAdd))
  (Default|SetScoreTexts (Variables|/Game/Blueprints/RythmePart/BP_RythmeSpline.BP_RythmeSpline_C|GetUI_Ref (Variables|References|GetRythmeSplineRef)) (select (> (Variables|Scoring|GetCombo) 0) (Math|Float|Truncate (* (Variables|Scoring|GetCombo) (Variables|Scoring|GetComboRatio) ScoreToAdd)) ScoreToAdd) NoteSuccess)
  (if (!= NoteSuccess 1)
    _
    (else
      (Variables|Scoring|SetComboRatio (Math|Float|Clamp(Float) (- (Variables|Scoring|GetComboRatio) 0.5) 1.5 5e+02))))
  (bind _result (Math|Integer|IncrementInt (Variables|Scoring|GetCombo))
    (:%20%20
      (Default|SetComboRangeCharacter _ui_ref)
      (Default|DisplayDancers _ui_ref)
      (Default|FeedbackGameplay _mainmenuref)
      (Default|FeedbackConfettis _mainmenuref)
      (Utilities|FlowControl|Sequence
        (:then_0
          (if (== (Math|Integer|%(Integer) _result 10) 0)
            (Variables|Scoring|SetComboRatio (+ (Variables|Scoring|GetComboRatio) 0.5))
            (if (Utilities|Struct|BreakS_Tracks (Variables|Default|GetSelectedTrack))
              (Variables|Default|SetNozomiScore (+ (Variables|Default|GetNozomiScore) 8))
              (else
                (Variables|Default|SetBokenScore (+ (Variables|Default|GetBokenScore) 8))))))
        (:then_1
          (if (> (Variables|Scoring|GetCombo) (Variables|Scoring|GetMaxCombo))
            (Variables|Scoring|SetMaxCombo (Variables|Scoring|GetCombo))))))))

(event Custom|SetAllVariablesToZero
  (bind _amountofeachnotesuccess (Variables|Scoring|GetAmountOfEachNoteSuccess))
  (bind _rythmesplineref (Variables|References|GetRythmeSplineRef))
  (bind _rythmesplineref_2 (Variables|References|GetRythmeSplineRef))
  (bind _ui_ref (Variables|/Game/Blueprints/RythmePart/BP_RythmeSpline.BP_RythmeSpline_C|GetUI_Ref _rythmesplineref_2))
  (bind _ui_ref_2 (Variables|/Game/Blueprints/RythmePart/BP_RythmeSpline.BP_RythmeSpline_C|GetUI_Ref _rythmesplineref))
  ;[0.15 0.15 0.15 0.5] Set all variables to zero
  (Variables|Scoring|SetScore 0)
  (Variables|Scoring|SetCombo 0)
  (Variables|Scoring|SetComboRatio 1.5)
  (Variables|Scoring|SetNotesHitted 0)
  (Variables|Scoring|SetMaxCombo 0)
  (Variables|Default|SetNozomiScore 0)
  (Variables|Default|SetBokenScore 0)
  (Variables|Scoring|SetRankScore 0)
  (Default|UpdateProgressBar _ui_ref_2)
  (Default|DisplayDancers _ui_ref_2)
  (Default|SetBaseCharacter _ui_ref_2)
  (Widget|SetVisibility (Variables|/Game/Blueprints/RythmePart/Widgets/WBP_Gameplay.WBP_Gameplay_C|GetWBP_AllAudioBars _ui_ref_2) "Collapsed")
  (Widget|SetVisibility (Variables|/Game/Blueprints/RythmePart/Widgets/WBP_MainMenu.WBP_MainMenu_C|GetOverlay_NoteIncoming (Variables|References|GetMainMenuRef)) "Hidden")
  (for (_ _array_index) _amountofeachnotesuccess
    (Utilities|Array|SetArrayElem _amountofeachnotesuccess _array_index 0 true)
    (Default|SetScoreTexts _ui_ref)
    (Rendering|Components|TextRender|SetText (Variables|/Game/Blueprints/RythmePart/Widgets/WBP_Gameplay.WBP_Gameplay_C|GetText_TrackProgress _ui_ref) "0 %")))

(event Custom|InputDelay
  ;[0.15 0.15 0.15 0.5] Input Delay
  (Variables|Default|SetCanEnterInput false)
  (Utilities|FlowControl|Delay 0.06)
  (Variables|Default|SetCanEnterInput true))

(event Input|EnhancedActionEvents|EnhancedInputActionIA_Left
  (params (ActionValue :type Boolean) (ElapsedSeconds :type Float%20%28double-precision%29) (TriggeredSeconds :type Float%20%28double-precision%29) (InputAction :type Input%20Action%20Object%20Reference :default "/Game/Blueprints/Core/Inputs/IA_Left.IA_Left"))
  (bind _rythmesplineref (Variables|References|GetRythmeSplineRef))
  (bind _sphere_left (Variables|/Game/Blueprints/RythmePart/BP_RythmeSpline.BP_RythmeSpline_C|GetSphere_Left _rythmesplineref))
  (bind _overlappingactors (Collision|GetOverlappingActors _sphere_left "/Game/Blueprints/RythmePart/BP_Note.BP_Note_C" :!class /Script/Engine.PrimitiveComponent))
  (bind _output (Utilities|Array|Get(acopy) _overlappingactors))
  (bind _asbp_note (Utilities|Casting|CastToBP_Note _output))
  ;[0.15 0.15 0.15 0.5] Inputs Directions
  (if (Variables|Default|GetCanEnterInput)
    (CallFunction|InputDelay)
    (Utilities|IsValid _rythmesplineref
      (:Is%20Valid
        (Default|PulsingEnteredInput _rythmesplineref "NewEnumerator0")
        (Utilities|IsValid _asbp_note
          (:Is%20Valid
            (Default|VerifyInput (Variables|References|GetRythmeSplineRef) (.x (- (Transformation|GetActorLocation _output) (Transformation|GetWorldLocation (Variables|/Game/Blueprints/RythmePart/BP_RythmeSpline.BP_RythmeSpline_C|GetArrow_Sphere_Left _rythmesplineref)))) _asbp_note)))))))

(event Input|EnhancedActionEvents|EnhancedInputActionIA_Reset
  (params (ActionValue :type Boolean) (ElapsedSeconds :type Float%20%28double-precision%29) (TriggeredSeconds :type Float%20%28double-precision%29) (InputAction :type Input%20Action%20Object%20Reference :default "/Game/Blueprints/Core/Inputs/IA_Reset.IA_Reset"))
  (bind _mainmenuref (Variables|References|GetMainMenuRef))
  (bind _rythmesplineref (Variables|References|GetRythmeSplineRef))
  (bind _mainmenuref_2 (Variables|References|GetMainMenuRef))
  ;[0.15 0.15 0.15 0.5] Input Reset Track
  (:Started
    (if (> (Variables|Scoring|GetNotesHitted) 0)
      (Variables|Default|SetIsResetting true)
      (Default|CallDestroyAllNotes)
      (Class|AudioParameterControllerInterface|SetTriggerParameter (Variables|/Game/Blueprints/RythmePart/BP_RythmeSpline.BP_RythmeSpline_C|GetAudio _rythmesplineref) "Stop")
      (Class|AudioParameterControllerInterface|SetTriggerParameter (Variables|/Game/Blueprints/RythmePart/BP_RythmeSpline.BP_RythmeSpline_C|GetAudioPreview _rythmesplineref) "Stop")
      (Components|Animation|PlayAnimation _mainmenuref_2 (Variables|/Game/Blueprints/RythmePart/Widgets/WBP_MainMenu.WBP_MainMenu_C|GetFadeToBlack _mainmenuref_2) 0.0
        (:Finished
          (CallFunction|SetAllVariablestoZero)
          (Components|Animation|PlayAnimation _mainmenuref (Variables|/Game/Blueprints/RythmePart/Widgets/WBP_MainMenu.WBP_MainMenu_C|GetFadeToBlack _mainmenuref) 0.0 1 "Reverse"
            (:Finished
              (Widget|SetVisibility (Variables|/Game/Blueprints/RythmePart/Widgets/WBP_MainMenu.WBP_MainMenu_C|GetImage_FadeToBlack (Variables|References|GetMainMenuRef)) "Collapsed")
              (Default|StartSequence (Variables|References|GetRythmeSplineRef)))))))))

(event Input|EnhancedActionEvents|EnhancedInputActionIA_Right
  (params (ActionValue :type Boolean) (ElapsedSeconds :type Float%20%28double-precision%29) (TriggeredSeconds :type Float%20%28double-precision%29) (InputAction :type Input%20Action%20Object%20Reference :default "/Game/Blueprints/Core/Inputs/IA_Right.IA_Right"))
  (bind _rythmesplineref (Variables|References|GetRythmeSplineRef))
  (bind _sphere_right (Variables|/Game/Blueprints/RythmePart/BP_RythmeSpline.BP_RythmeSpline_C|GetSphere_Right _rythmesplineref))
  (bind _overlappingactors (Collision|GetOverlappingActors _sphere_right "/Game/Blueprints/RythmePart/BP_Note.BP_Note_C" :!class /Script/Engine.PrimitiveComponent))
  (bind _output (Utilities|Array|Get(acopy) _overlappingactors))
  (bind _asbp_note (Utilities|Casting|CastToBP_Note _output))
  ;[0.15 0.15 0.15 0.5] Inputs Directions
  (if (Variables|Default|GetCanEnterInput)
    (CallFunction|InputDelay)
    (Utilities|IsValid _rythmesplineref
      (:Is%20Valid
        (Default|PulsingEnteredInput _rythmesplineref "NewEnumerator3")
        (Utilities|IsValid _asbp_note
          (:Is%20Valid
            (Default|VerifyInput (Variables|References|GetRythmeSplineRef) (.x (- (Transformation|GetActorLocation _output) (Transformation|GetWorldLocation (Variables|/Game/Blueprints/RythmePart/BP_RythmeSpline.BP_RythmeSpline_C|GetArrow_Sphere_Right _rythmesplineref)))) _asbp_note)))))))

(event Input|EnhancedActionEvents|EnhancedInputActionIA_Up
  (params (ActionValue :type Boolean) (ElapsedSeconds :type Float%20%28double-precision%29) (TriggeredSeconds :type Float%20%28double-precision%29) (InputAction :type Input%20Action%20Object%20Reference :default "/Game/Blueprints/Core/Inputs/IA_Up.IA_Up"))
  (bind _rythmesplineref (Variables|References|GetRythmeSplineRef))
  (bind _sphere_top (Variables|/Game/Blueprints/RythmePart/BP_RythmeSpline.BP_RythmeSpline_C|GetSphere_Top _rythmesplineref))
  (bind _overlappingactors (Collision|GetOverlappingActors _sphere_top "/Game/Blueprints/RythmePart/BP_Note.BP_Note_C" :!class /Script/Engine.PrimitiveComponent))
  (bind _output (Utilities|Array|Get(acopy) _overlappingactors))
  (bind _asbp_note (Utilities|Casting|CastToBP_Note _output))
  ;[0.15 0.15 0.15 0.5] Inputs Directions
  (if (Variables|Default|GetCanEnterInput)
    (CallFunction|InputDelay)
    (Utilities|IsValid _rythmesplineref
      (:Is%20Valid
        (Default|PulsingEnteredInput _rythmesplineref "NewEnumerator2")
        (Utilities|IsValid _asbp_note
          (:Is%20Valid
            (Default|VerifyInput (Variables|References|GetRythmeSplineRef) (.x (- (Transformation|GetActorLocation _output) (Transformation|GetWorldLocation (Variables|/Game/Blueprints/RythmePart/BP_RythmeSpline.BP_RythmeSpline_C|GetArrow_Sphere_Top _rythmesplineref)))) _asbp_note)))))))

(event Input|EnhancedActionEvents|EnhancedInputActionIA_Down
  (params (ActionValue :type Boolean) (ElapsedSeconds :type Float%20%28double-precision%29) (TriggeredSeconds :type Float%20%28double-precision%29) (InputAction :type Input%20Action%20Object%20Reference :default "/Game/Blueprints/Core/Inputs/IA_Down.IA_Down"))
  (bind _rythmesplineref (Variables|References|GetRythmeSplineRef))
  (bind _sphere_bottom (Variables|/Game/Blueprints/RythmePart/BP_RythmeSpline.BP_RythmeSpline_C|GetSphere_Bottom _rythmesplineref))
  (bind _overlappingactors (Collision|GetOverlappingActors _sphere_bottom "/Game/Blueprints/RythmePart/BP_Note.BP_Note_C" :!class /Script/Engine.PrimitiveComponent))
  (bind _output (Utilities|Array|Get(acopy) _overlappingactors))
  (bind _asbp_note (Utilities|Casting|CastToBP_Note _output))
  ;[0.15 0.15 0.15 0.5] Inputs Directions
  (if (Variables|Default|GetCanEnterInput)
    (CallFunction|InputDelay)
    (Utilities|IsValid _rythmesplineref
      (:Is%20Valid
        (Default|PulsingEnteredInput _rythmesplineref "NewEnumerator1")
        (Utilities|IsValid _asbp_note
          (:Is%20Valid
            (Default|VerifyInput (Variables|References|GetRythmeSplineRef) (.x (- (Transformation|GetActorLocation _output) (Transformation|GetWorldLocation (Variables|/Game/Blueprints/RythmePart/BP_RythmeSpline.BP_RythmeSpline_C|GetArrow_Sphere_Bottom _rythmesplineref)))) _asbp_note)))))))

(event Input|EnhancedActionEvents|EnhancedInputActionIA_Quit
  (params (ActionValue :type Boolean) (ElapsedSeconds :type Float%20%28double-precision%29) (TriggeredSeconds :type Float%20%28double-precision%29) (InputAction :type Input%20Action%20Object%20Reference :default "/Game/Blueprints/Core/Inputs/IA_Quit.IA_Quit"))
  (bind _mainmenuref (Variables|References|GetMainMenuRef))
  (bind _mainmenuref_2 (Variables|References|GetMainMenuRef))
  (bind _rythmesplineref (Variables|References|GetRythmeSplineRef))
  (bind _mainmenuref_3 (Variables|References|GetMainMenuRef))
  ;[0.15 0.15 0.15 0.5] Input Quit Track
  (:Started
    (if (Variables|/Game/Blueprints/RythmePart/BP_RythmeSpline.BP_RythmeSpline_C|GetIsSoundStarting (Variables|References|GetRythmeSplineRef))
      (Variables|Default|SetIsResetting true)
      (Default|CallDestroyAllNotes)
      (Class|AudioParameterControllerInterface|SetTriggerParameter (Variables|/Game/Blueprints/RythmePart/BP_RythmeSpline.BP_RythmeSpline_C|GetAudio _rythmesplineref) "Stop")
      (Class|AudioParameterControllerInterface|SetTriggerParameter (Variables|/Game/Blueprints/RythmePart/BP_RythmeSpline.BP_RythmeSpline_C|GetAudioPreview _rythmesplineref) "Stop")
      (Components|Animation|PlayAnimation _mainmenuref (Variables|/Game/Blueprints/RythmePart/Widgets/WBP_MainMenu.WBP_MainMenu_C|GetFadeToBlack _mainmenuref) 0.0
        (:Finished
          (Default|FinishSequence (Variables|References|GetRythmeSplineRef))
          (Input|SetInputModeUIOnly self (Variables|References|GetMainMenuRef) "DoNotLock" true)
          (Variables|Default|SetbShowMouseCursor true)
          (Default|CheckSelectedTrack _mainmenuref_2)
          (Default|SetPreviewSound _mainmenuref_2)
          (Class|WidgetSwitcher|SetActiveWidgetIndex (Variables|/Game/Blueprints/RythmePart/Widgets/WBP_MainMenu.WBP_MainMenu_C|GetWS_MainMenu _mainmenuref_2) 1)
          (Components|Animation|PlayAnimation _mainmenuref_3 (Variables|/Game/Blueprints/RythmePart/Widgets/WBP_MainMenu.WBP_MainMenu_C|GetPopUp_TrackSelection _mainmenuref_3) 0.0
            (:Finished
              (Default|DisplayCurrentTrack _mainmenuref_2))))))))

(event EventBeginPlay
  (bind _self self)
  (bind _returnvalue (PlayerController|LocalPlayerSubsystems|GetEnhancedInputLocalPlayerSubsystem _self))
  (bind _returnvalue_2 (Class|EnhancedInputSubsystemInterface|GetUserSettings _returnvalue))
  ;[0.15 0.15 0.15 0.5] Begin Play
  (Utilities|FlowControl|Sequence
    (:then_0
      (Input|AddMappingContext _returnvalue "/Game/Blueprints/Core/IMC_Base.IMC_Base" 0 "(bIgnoreAllPressedKeysUntilRelease=True,bForceImmediately=False,bNotifyUserSettings=False)")
      (if (not (Class|EnhancedInputUserSettings|IsMappingContextRegistered _returnvalue_2 "/Game/Blueprints/Core/IMC_Base.IMC_Base"))
        (Class|EnhancedInputUserSettings|RegisterInputMappingContext _returnvalue_2 "/Game/Blueprints/Core/IMC_Base.IMC_Base")))
    (:then_1
      (bind _returnvalue_3 (UserInterface|CreateWidget "/Game/Blueprints/RythmePart/Widgets/Menus/WBP_Intro.WBP_Intro_C"))
      (UserInterface|Viewport|AddtoViewport _returnvalue_3 0))))

(fn ConstructionScript)

(fn CalculateHigherScorePossible
  (return (* (.NumberOfNotes (Utilities|Struct|BreakS_Tracks (Variables|Default|GetSelectedTrack))) 500)))

(fn VerifyRankObtained
  (bind _higherscorepossible (CallFunction|CalculateHigherScorePossible))
  (return (select (== (Variables|Scoring|GetRankScore) _higherscorepossible) 6 (select (>= (Variables|Scoring|GetRankScore) (Math|Float|Truncate (* (Math|Conversions|ToFloat(Integer) _higherscorepossible) 0.95))) 5 (select (>= (Variables|Scoring|GetRankScore) (Math|Float|Truncate (* (Math|Conversions|ToFloat(Integer) _higherscorepossible) 0.9))) 4 (select (>= (Variables|Scoring|GetRankScore) (Math|Float|Truncate (* (Math|Conversions|ToFloat(Integer) _higherscorepossible) 0.8))) 3 (select (>= (Variables|Scoring|GetRankScore) (Math|Float|Truncate (* (Math|Conversions|ToFloat(Integer) _higherscorepossible) 0.6))) 2 (select (>= (Variables|Scoring|GetRankScore) (Math|Float|Truncate (* (Math|Conversions|ToFloat(Integer) _higherscorepossible) 0.4))) 1 0))))))))