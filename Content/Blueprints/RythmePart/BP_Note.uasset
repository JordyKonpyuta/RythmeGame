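; Rhythm-game arrow note that travels along one of SplineRef's four lane splines, chosen by NoteType.
; BeginPlay orients and colors the arrow by type, then a timeline moves it along the spline, calling FailedNote past a fixed world X.
; A second timeline, PulsingNote, increments mesh roll.
; It binds to and fires the player controller's DestroyAllNotes event on spawn, destroying itself only while IsResetting is true.
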(event Custom|DestroyNote
  (if (Variables|/Game/Blueprints/Core/BP_RythmeGameController.BP_RythmeGameController_C|GetIsResetting (Variables|/Game/Blueprints/RythmePart/BP_RythmeSpline.BP_RythmeSpline_C|GetPlayerController (Variables|Default|GetSplineRef)))
    (Actor|DestroyActor)))

(event EventBeginPlay
  (bind _splineref (Variables|Default|GetSplineRef))
  (bind _notetype (Variables|Default|GetNoteType))
  (bind _staticmesh (Variables|Default|GetStaticMesh))
  (bind _spline_bottom (Variables|/Game/Blueprints/RythmePart/BP_RythmeSpline.BP_RythmeSpline_C|GetSpline_Bottom _splineref))
  (bind _relativerotation (Variables|/Script/Engine.SceneComponent|GetRelativeRotation _staticmesh))
  (bind _spline_left (Variables|/Game/Blueprints/RythmePart/BP_RythmeSpline.BP_RythmeSpline_C|GetSpline_Left _splineref))
  (bind _spline_right (Variables|/Game/Blueprints/RythmePart/BP_RythmeSpline.BP_RythmeSpline_C|GetSpline_Right _splineref))
  (bind _spline_top (Variables|/Game/Blueprints/RythmePart/BP_RythmeSpline.BP_RythmeSpline_C|GetSpline_Top _splineref))
  (bind _returnvalue (Utilities|Select :Index _notetype :NewEnumerator0 _spline_left :NewEnumerator1 _spline_bottom :NewEnumerator2 _spline_top :NewEnumerator3 _spline_right))
  (Utilities|FlowControl|Sequence
    (:then_0
      (EventDispatchers|BindEventtoDestroyAllNotes (Variables|/Game/Blueprints/RythmePart/BP_RythmeSpline.BP_RythmeSpline_C|GetPlayerController (Variables|Default|GetSplineRef)) (delegate Custom|DestroyNote)))
    (:then_1
      (Default|CallDestroyAllNotes (Variables|/Game/Blueprints/RythmePart/BP_RythmeSpline.BP_RythmeSpline_C|GetPlayerController (Variables|Default|GetSplineRef)))
      (Transformation|SetRelativeRotation (Variables|Default|GetStaticMesh) (Utilities|Select :Index (Variables|Default|GetNoteType) :NewEnumerator0 "180.000000,0.000000,90.000000" :NewEnumerator1 "-90.000000,0.000000,90.000000" :NewEnumerator2 "90.000000,0.000000,90.000000" :NewEnumerator3 "0.000000,0.000000,90.000000") false false)
      (Rendering|Material|SetMaterial (Variables|Default|GetStaticMesh) 0 (Utilities|Select :Index (Variables|Default|GetNoteType) :NewEnumerator0 "/Game/Assets/Models/MI_Arrow_Left.MI_Arrow_Left" :NewEnumerator1 "/Game/Assets/Models/MI_Arrow_Bottom.MI_Arrow_Bottom" :NewEnumerator2 "/Game/Assets/Models/MI_Arrow_Top.MI_Arrow_Top" :NewEnumerator3 "/Game/Assets/Models/MI_Arrow_Right.MI_Arrow_Right"))
      (Utilities|IsValid _splineref
        (:Is%20Valid
          (bind _newtrack_0 (Timeline|MoveNote Play)
            (:Update
              (Transformation|SetActorTransform (Math|Transform|MakeTransform (Math|Vector|MakeVector (.x (Spline|GetLocationatDistanceAlongSpline _returnvalue (Math|Float|Lerp 0.0 (Spline|GetSplineLength _returnvalue) _newtrack_0) "World")) (.y (Spline|GetLocationatDistanceAlongSpline _returnvalue (Math|Float|Lerp 0.0 (Spline|GetSplineLength _returnvalue) _newtrack_0) "World")) (.z (Spline|GetLocationatDistanceAlongSpline _returnvalue (Math|Float|Lerp 0.0 (Spline|GetSplineLength _returnvalue) _newtrack_0) "World"))) "0, 0, 0" "1.200000,1.200000,1.200000"))
              (if (>= (.x (Spline|GetLocationatDistanceAlongSpline _returnvalue (Math|Float|Lerp 0.0 (Spline|GetSplineLength _returnvalue) _newtrack_0) "World")) 3.4e+03)
                (Default|FailedNote (Variables|Default|GetSplineRef) self)))))))
    (:then_2
      (bind _notesize (Timeline|PulsingNote Play)
        (:Update
          (Transformation|SetRelativeRotation _staticmesh (Math|Rotator|MakeRotator (+ (.roll _relativerotation) _notesize) (.pitch _relativerotation) (.yaw _relativerotation)) false false))))))

(fn ConstructionScript)