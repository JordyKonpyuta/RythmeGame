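; BP_RythmeSpline is the rhythm game's note track, spawning notes, judging inputs and triggering end-of-track display.
; A muted MetaSound copy starts first, its watched cue points spawning BP_Note at four directional arrows.
; The audible copy follows after a fixed delay, driving audio-bar visualisation through playback time.
; Distance-based judging updates score, hit tallies and widget feedback, with misses resetting combo; a timeline pulses input planes.
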(event Custom|StartSequence
  (bind _playercontroller (Variables|Default|GetPlayerController))
  (bind _selectedtrack (Variables|/Game/Blueprints/Controller/BP_RythmeGameController.BP_RythmeGameController_C|GetSelectedTrack _playercontroller))
  (bind _trackingame (Utilities|Struct|BreakS_Tracks _selectedtrack))
  ;[0.15 0.15 0.15 0.5] Start Sequence
  (Default|CallDestroyAllNotes (Variables|Default|GetPlayerController))
  (Utilities|FlowControl|Sequence
    (:then_0
      (Utilities|FlowControl|Delay 2.25)
      (bind _returnvalue (AddComponent|AddAudioComponent false))
      (bind _output_get (Variables|Default|SetAudioPreview _returnvalue))
      (Class|AudioComponent|SetWaveParameter _output_get "Wave Asset" _trackingame)
      (Class|AudioParameterControllerInterface|SetTriggerParameter _output_get "On Play")
      (Widget|SetVisibility (Variables|/Game/Blueprints/RythmePart/WBP_Gameplay.WBP_Gameplay_C|GetWBP_AllAudioBars (Variables|Default|GetUI_Ref)) "SelfHitTestInvisible")
      (Variables|/Game/Blueprints/Controller/BP_RythmeGameController.BP_RythmeGameController_C|SetIsResetting (Variables|Default|GetPlayerController) false)
      (MetaSoundOutput|WatchOutput (WorldSubsystems|GetMetaSoundOutputSubsystem) (Variables|Default|GetAudioPreview) "Playback Time" (delegate Custom|AudioReaction) "None" "None" :!class /Script/MetasoundEngine.MetaSoundOutputSubsystem))
    (:then_1
      (bind _returnvalue_2 (AddComponent|AddAudioComponent false))
      (bind _output_get_2 (Variables|Default|SetAudio _returnvalue_2))
      (Class|AudioComponent|SetWaveParameter _output_get_2 "Wave Asset" _trackingame)
      (Class|AudioParameterControllerInterface|SetTriggerParameter _output_get_2 "On Play")
      (Audio|Components|Audio|SetVolumeMultiplier _output_get_2 0.0 :!class /Script/Engine.AudioComponent)
      (MetaSoundOutput|WatchOutput (WorldSubsystems|GetMetaSoundOutputSubsystem) (Variables|Default|GetAudio) "CuePoint_Direction" (delegate Custom|SpawnNoteOnGoodLine) "None" "None" :!class /Script/MetasoundEngine.MetaSoundOutputSubsystem)
      (EventDispatchers|BindEventtoOnAudioFinished (Variables|Default|GetAudio) (delegate Custom|FinishSequence)))))

(event Custom|SpawnNoteOnGoodLine
  (params (OutputName :type Name) (Output :type Meta%20Sound%20Output%20Structure%20%28by%20ref%29))
  ;[0.15 0.15 0.15 0.5] Start Sequence
  (bind _returnvalue (Class|MetasoundOutputBlueprintAccess|GetString Output))
  (for (_array_element _array_index) (Utilities|Array|MakeArray (Utilities|Enum|Equal(Enum) (.RightS (Utilities|String|Split _returnvalue "_")) "Top") (Utilities|Enum|Equal(Enum) (.RightS (Utilities|String|Split _returnvalue "_")) "Bottom") (Utilities|Enum|Equal(Enum) (.RightS (Utilities|String|Split _returnvalue "_")) "Right") (Utilities|Enum|Equal(Enum) (.RightS (Utilities|String|Split _returnvalue "_")) "Left"))
    (if _array_element
      (Game|SpawnActorfromClass "/Game/Blueprints/RythmePart/BP_Note.BP_Note_C" (Transformation|GetWorldTransform (Utilities|Array|Get(acopy) (Utilities|Array|MakeArray (Variables|Default|GetArrow_Top) (Variables|Default|GetArrow_Bottom) (Variables|Default|GetArrow_Right) (Variables|Default|GetArrow_Left)) _array_index)) "Undefined" "MultiplyWithRoot" 0 (Utilities|Select :Index _array_index :Option%200 "NewEnumerator2" :Option%201 "NewEnumerator1" :Option%202 "NewEnumerator3" :Option%203 "NewEnumerator0") self 0))))

(event Custom|AudioReaction
  (params (OutputName :type Name) (Output :type Meta%20Sound%20Output%20Structure%20%28by%20ref%29))
  (bind _ui_ref (Variables|Default|GetUI_Ref))
  ;[0.15 0.15 0.15 0.5] Start Sequence
  (bind _returnvalue (Utilities|Time|GetTimeSeconds Output))
  (Default|AudioVisualisationforAllBars (Variables|/Game/Blueprints/RythmePart/WBP_Gameplay.WBP_Gameplay_C|GetWBP_AllAudioBars _ui_ref) (Utilities|Array|Get(acopy) (Variables|/Game/Blueprints/RythmePart/WBP_Gameplay.WBP_Gameplay_C|GetInGameNRT _ui_ref) (Variables|/Game/Blueprints/RythmePart/WBP_MainMenu.WBP_MainMenu_C|GetIndex (Variables|/Game/Blueprints/Controller/BP_RythmeGameController.BP_RythmeGameController_C|GetMainMenuRef (Variables|Default|GetPlayerController)))) (* _returnvalue (Variables|/Script/Engine.SoundBase|GetDuration (Variables|/Script/Engine.AudioComponent|GetSound (Variables|Default|GetAudioPreview))))))

(event Custom|SetFeedback
  (params (NoteToCheck :type BP%20Note%20Object%20Reference) (SuccessRate :type Integer))
  ;[0.15 0.15 0.15 0.5] Note's Feedback
  (Utilities|IsValid NoteToCheck
    (:Is%20Valid
      (Default|DisplayFeedback (.AsWBP%20Note%20Feedback (Utilities|Casting|CastToWBP_NoteFeedback (UserInterface|GetWidget (Utilities|Select :Index (Variables|/Game/Blueprints/RythmePart/BP_Note.BP_Note_C|GetNoteType NoteToCheck) :NewEnumerator0 (Variables|Default|GetWidget_Feedback_Left) :NewEnumerator1 (Variables|Default|GetWidget_Feedback_Bottom) :NewEnumerator2 (Variables|Default|GetWidget_Feedback_Top) :NewEnumerator3 (Variables|Default|GetWidget_Feedback_Right))))) SuccessRate)
      (for _array_element (Utilities|Array|MakeArray (Variables|Default|GetWidget_Feedback_Left) (Variables|Default|GetWidget_Feedback_Bottom) (Variables|Default|GetWidget_Feedback_Top) (Variables|Default|GetWidget_Feedback_Right))
        (Default|SetFireVisibility (.AsWBP%20Note%20Feedback (Utilities|Casting|CastToWBP_NoteFeedback (UserInterface|GetWidget _array_element))))))))

(event Custom|VerifyInput
  (params (Distance :type Float%20%28double-precision%29) (NoteToVerify :type BP%20Note%20Object%20Reference))
  (bind _returnvalue (Math|Float|Absolute(Float) Distance))
  ;[0.15 0.15 0.15 0.5] Verify Input Result
  (if (<= _returnvalue 35.0)
    (Default|AddScore (Variables|Default|GetPlayerController) 500)
    (CallFunction|SetFeedback NoteToVerify 3)
    (Actor|DestroyActor NoteToVerify)
    (CallFunction|IncrementeNoteAmount)
    (elif (and (> _returnvalue 35.0) (<= _returnvalue 65.0))
      (Default|AddScore (Variables|Default|GetPlayerController) 300)
      (CallFunction|SetFeedback NoteToVerify 2)
      (Actor|DestroyActor NoteToVerify)
      (CallFunction|IncrementeNoteAmount 1)
      (elif (and (> _returnvalue 65.0) (<= _returnvalue 1.6e+02))
        (Default|AddScore (Variables|Default|GetPlayerController) 100)
        (CallFunction|SetFeedback NoteToVerify 1)
        (Actor|DestroyActor NoteToVerify)
        (CallFunction|IncrementeNoteAmount 2)
        (else
          (CallFunction|FailedNote NoteToVerify)
          (CallFunction|SetFeedback NoteToVerify))))))

(event Custom|IncrementeNoteAmount
  (params (IndexToIncremente :type Integer))
  (bind _playercontroller (Variables|Default|GetPlayerController))
  (bind _amountofeachnotesuccess (Variables|/Game/Blueprints/Controller/BP_RythmeGameController.BP_RythmeGameController_C|GetAmountOfEachNoteSuccess _playercontroller))
  ;[0.15 0.15 0.15 0.5] Incremente Note Amount
  (Utilities|Array|SetArrayElem _amountofeachnotesuccess IndexToIncremente (+ (Utilities|Array|Get(acopy) _amountofeachnotesuccess IndexToIncremente) 1) true)
  (Math|Integer|IncrementInt (Variables|/Game/Blueprints/Controller/BP_RythmeGameController.BP_RythmeGameController_C|GetNotesHitted (Variables|Default|GetPlayerController))
    (:%20%20
      (Default|UpdateProgressBar (Variables|Default|GetUI_Ref)))))

(event Custom|FailedNote
  (params (NoteFailed :type BP%20Note%20Object%20Reference))
  (bind _playercontroller (Variables|Default|GetPlayerController))
  ;[0.15 0.15 0.15 0.5] Failed Note
  (Default|AddScore (Variables|Default|GetPlayerController))
  (CallFunction|SetFeedback NoteFailed)
  (Actor|DestroyActor NoteFailed)
  (Variables|/Game/Blueprints/Controller/BP_RythmeGameController.BP_RythmeGameController_C|SetCombo _playercontroller 0)
  (Variables|/Game/Blueprints/Controller/BP_RythmeGameController.BP_RythmeGameController_C|SetComboRatio _playercontroller 1.5)
  (Default|SetFailCharacter (Variables|Default|GetUI_Ref))
  (CallFunction|IncrementeNoteAmount 3))

(event Custom|FinishSequence
  (bind _playercontroller (Variables|Default|GetPlayerController))
  (bind _mainmenuref (Variables|/Game/Blueprints/Controller/BP_RythmeGameController.BP_RythmeGameController_C|GetMainMenuRef _playercontroller))
  ;[0.15 0.15 0.15 0.5] Start Sequence
  (if (not (Variables|/Game/Blueprints/Controller/BP_RythmeGameController.BP_RythmeGameController_C|GetIsResetting (Variables|Default|GetPlayerController)))
    (Utilities|FlowControl|Delay 5.0)
    (Widget|SetVisibility _mainmenuref "SelfHitTestInvisible")
    (Default|DisplayEndTrack _mainmenuref)
    (Input|SetInputModeUIOnly (Variables|Default|GetPlayerController) _mainmenuref "DoNotLock" true)
    (Variables|/Script/Engine.PlayerController|SetbShowMouseCursor (Variables|Default|GetPlayerController) true)))

(event Custom|PulsingEnteredInput
  (params (InputEntered :type E_NoteType%20Enum :default "NewEnumerator0"))
  ;[0.15 0.15 0.15 0.5] Pulsing Entered Input
  (bind _inputsize (Timeline|PulsingInput PlayFromStart)
    (:Update
      (Transformation|SetWorldScale3D (Utilities|Select :Index InputEntered :NewEnumerator0 (Variables|Default|GetPlane_Left) :NewEnumerator1 (Variables|Default|GetPlane_Bottom) :NewEnumerator2 (Variables|Default|GetPlane_Top) :NewEnumerator3 (Variables|Default|GetPlane_Right)) (Math|Conversions|ToVector(Float) _inputsize)))))

(event EventBeginPlay
  ;[0.15 0.15 0.15 0.5] Begin Play
  (Variables|Default|SetUI_Ref (.AsWBP%20Gameplay (Utilities|Casting|CastToWBP_Gameplay (UserInterface|GetWidget (Variables|Default|GetWidget_Gameplay)))))
  (bind _asbp_rythme_game_controller (Utilities|Casting|CastToBP_RythmeGameController (Game|GetPlayerController 0)))
  (bind _output_get (Variables|Default|SetPlayerController _asbp_rythme_game_controller))
  (Variables|/Game/Blueprints/Controller/BP_RythmeGameController.BP_RythmeGameController_C|SetRythmeSplineRef _output_get self))

(fn ConstructionScript)